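; Bomb pickup actor that awards score and bombs to the BP_Nave_Proposta2 that touches it.
; A capsule overlap adds a fixed score, increments the Bomba count while it is below its cap, then destroys the pickup, even if the count is full.
; Tick rewrites the PickUp component's relative rotation with a zero roll increment, so it produces no spin.
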(event `self.ReceiveBeginPlay`)

(event `self.ReceiveTick`
  (params (DeltaSeconds :type "Float (single-precision)"))
  (bind _pickup (`self.PickUp`))
  (bind (_relativerotation_roll _relativerotation_pitch _relativerotation_yaw) (`KismetMathLibrary.BreakRotator` (`SceneComponent.RelativeRotation` _pickup)))
  (`SceneComponent.K2_SetRelativeRotation` _pickup (`KismetMathLibrary.MakeRotator` (+ _relativerotation_roll 0.0) _relativerotation_pitch _relativerotation_yaw) false false))

(event `self.Capsule.OnComponentBeginOverlap`
  (params (OverlappedComponent :type "PrimitiveComponent Object Reference") (OtherActor :type "Actor Object Reference") (OtherComp :type "PrimitiveComponent Object Reference") (OtherBodyIndex :type Integer) (bFromSweep :type Boolean) (SweepResult :type "HitResult Structure (by ref)"))
  (bind _asbp_nave_proposta_2 (cast `/Game/NAVE_PROPOSTA/BP_Nave_Proposta2` OtherActor))
  (set `/Game/NAVE_PROPOSTA/BP_Nave_Proposta2.Score` (+ (`/Game/NAVE_PROPOSTA/BP_Nave_Proposta2.Score` _asbp_nave_proposta_2) 200) _asbp_nave_proposta_2)
  (bind _bomba (`/Game/NAVE_PROPOSTA/BP_Nave_Proposta2.Bomba` _asbp_nave_proposta_2))
  (if (<= _bomba 2)
    (set `/Game/NAVE_PROPOSTA/BP_Nave_Proposta2.Bomba` (+ _bomba 1) _asbp_nave_proposta_2))
  (`self.K2_DestroyActor`))

(fn `UserConstructionScript`)