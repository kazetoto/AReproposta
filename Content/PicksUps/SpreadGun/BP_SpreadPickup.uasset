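; BP_SpreadPickup is a collectible pickup that gives the player airship the spread gun pickup type.
; When the player pawn overlaps its Capsule, it casts to BP_PlayerAirship, adds score, sets PickupTypes, prints the new value and destroys itself.
; Tick re-applies the PickUp component's relative rotation with a zero roll increment, so it adds no visible spin.
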(event `self.ReceiveBeginPlay`)

(event `self.ReceiveTick`
  (params (DeltaSeconds :type "Float (single-precision)"))
  (bind _pickup (`self.PickUp`))
  (bind (_relativerotation_roll _relativerotation_pitch _relativerotation_yaw) (`KismetMathLibrary.BreakRotator` (`SceneComponent.RelativeRotation` _pickup)))
  (`SceneComponent.K2_SetRelativeRotation` _pickup (`KismetMathLibrary.MakeRotator` (+ _relativerotation_roll 0.0) _relativerotation_pitch _relativerotation_yaw) false false))

(event `self.Capsule.OnComponentBeginOverlap`
  (params (OverlappedComponent :type "PrimitiveComponent Object Reference") (OtherActor :type "Actor Object Reference") (OtherComp :type "PrimitiveComponent Object Reference") (OtherBodyIndex :type Integer) (bFromSweep :type Boolean) (SweepResult :type "HitResult Structure (by ref)"))
  (if (== OtherActor (`GameplayStatics.GetPlayerPawn` 0))
    (bind _asbp_player_airship (cast `/Game/PlayerAirship/BP_PlayerAirship` OtherActor))
    (set `/Game/PlayerAirship/BP_PlayerAirship.Score` (+ (`/Game/PlayerAirship/BP_PlayerAirship.Score` _asbp_player_airship) 200) _asbp_player_airship)
    (bind _output_get (set `/Game/PlayerAirship/BP_PlayerAirship.PickupTypes` 2 _asbp_player_airship))
    (`KismetSystemLibrary.PrintString` (`KismetStringLibrary.Conv_IntToString` _output_get))
    (`self.K2_DestroyActor`)))

(fn `UserConstructionScript`)