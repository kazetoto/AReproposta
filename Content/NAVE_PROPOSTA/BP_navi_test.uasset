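; Test ship Blueprint that moves on the X/Y plane from two input axes and banks as it moves sideways.
; Both axis events pass through a shared Movement function that eases each speed toward MovementSpeed times input with FInterpTo, using delta time cached from Tick.
; Tick applies the speeds as a swept per-frame location offset, unscaled by delta time, and rotates toward a roll derived from horizontal speed.
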(event `self.ReceiveTick`
  (params (DeltaSeconds :type "Float (single-precision)"))
  ;[0.1006 0 1] Movement
  (`|ExecutionSequence`
    (:`then_0`
      (set `self.DeltaSeconds` DeltaSeconds)
      (`self.K2_SetActorLocation` (+ (`self.K2_GetActorLocation`) (`KismetMathLibrary.MakeVector` (`self.VertSpeed`) (`self.HozSpeed`))) true)
      (`self.K2_SetActorRotation` (`KismetMathLibrary.RInterpTo_Constant` (`self.K2_GetActorRotation`) (`KismetMathLibrary.MakeRotator` (+ (* (`self.HozSpeed`) 7.0) (`self.Roll`))) (`self.DeltaSeconds`) 800.0)))))

(event `InputAxis|Mover_Cima_Embaixo`
  (params (AxisValue :type "Float (single-precision)"))
  ;[0.04042 1 0] Player input
  (bind _returndirectionspeed (`self.Movement` (`self.VertSpeed`) AxisValue))
  (set `self.VertSpeed` _returndirectionspeed))

(event `InputAxis|Mover`
  (params (AxisValue :type "Float (single-precision)"))
  ;[0.04042 1 0] Player input
  (bind _returndirectionspeed (`self.Movement` (`self.HozSpeed`) AxisValue))
  (set `self.HozSpeed` _returndirectionspeed))

(fn `Movement`
  (params (Speed :type "Float (double-precision)") (Direction :type "Float (double-precision)"))
  (returns (ReturnDirectionSpeed :type "Float (double-precision)"))
  (return (`KismetMathLibrary.FInterpTo` Speed (* (`self.MovementSpeed`) Direction) (`self.DeltaSeconds`) 6.0)))

(fn `UserConstructionScript`)