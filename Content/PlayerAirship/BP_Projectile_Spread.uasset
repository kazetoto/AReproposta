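; Spread-shot projectile for the player airship that damages what it overlaps and expires after about one second.
; The construction script creates a dynamic material and applies configurable scale and speed; BeginPlay sets the material colour.
; Overlap on the Tiro component applies damage, spawns a sparks-and-explosion emitter without auto-destroy, then destroys the projectile.
; Lifetime comes from a Delay on Tick leading to DestroyActor.
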(event `self.ReceiveBeginPlay`
  (`MaterialInstanceDynamic.SetVectorParameterValue` (`self.ProjectileMaterial`) "Colour" (`self.ProjectileColour`)))

(event `self.ReceiveTick`
  (params (DeltaSeconds :type "Float (single-precision)"))
  (`KismetSystemLibrary.Delay` 1.0)
  (`self.K2_DestroyActor` self :!label _label))

(event `self.Tiro.OnComponentBeginOverlap`
  (params (OverlappedComponent :type "PrimitiveComponent Object Reference") (OtherActor :type "Actor Object Reference") (OtherComp :type "PrimitiveComponent Object Reference") (OtherBodyIndex :type Integer) (bFromSweep :type Boolean) (SweepResult :type "HitResult Structure (by ref)"))
  (`GameplayStatics.ApplyDamage` OtherActor (`self.Damage`))
  (`GameplayStatics.SpawnEmitterAtLocation` "/Game/Particle/P_Sparks_With_Explosions.P_Sparks_With_Explosions" (`self.K2_GetActorLocation`) (struct) (1.0 1.0 1.0) false)
  (goto _label))

(fn `UserConstructionScript`
  (bind _projectilemovement (`self.ProjectileMovement`))
  (bind _returnvalue (`PrimitiveComponent.CreateDynamicMaterialInstance` (`self.Tiro`) 0 null "None"))
  (set `self.ProjectileMaterial` _returnvalue)
  (`SceneComponent.SetWorldScale3D` (`self.Tiro`) (`self.Scale`))
  (bind _output_get (set `ProjectileMovementComponent.MaxSpeed` (`self.Speed`) _projectilemovement))
  (set `ProjectileMovementComponent.InitialSpeed` _output_get _projectilemovement))