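; Player airship pawn for a shooter, with health, weapons, bombs and a pause menu.
; A spawn timeline plays a roll, then Tick moves and banks the ship from smoothed input speeds, bouncing it off hits.
; Gated DoOnce delays rate-limit default, machine-gun or spread fire by pickup type, plus limited bombs.
; Damage grants brief invincibility; death, or an expired countdown with negative score, calls game over on the GameMode.
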(event `self.ReceiveBeginPlay`
  ;[1 0.8776 0.08731] SpawnAnimation
  (bind _asgame_mode_bp (cast `/Game/Blueprints/GameMode_BP` (`GameplayStatics.GetGameMode`)))
  (set `self.BP_GameMode` _asgame_mode_bp)
  (set `self.Roll` (.yaw (`self.K2_GetActorRotation`)))
  (set `self.SpawnLocation` (`self.K2_GetActorLocation`))
  (bind (_direction _speed) (`Timeline|SpawnAnimation`)
    (:`Update`
      (`self.K2_SetActorLocation` (`self.SpawnLocation`))
      (`self.K2_SetActorRotation` (`KismetMathLibrary.RLerp` (struct) (`KismetMathLibrary.MakeRotator` (+ (`self.Roll`) 1440.0)) _speed)))))

(event `self.ReceiveTick`
  (params (DeltaSeconds :type "Float (single-precision)"))
  ;[0.1006 0 1] Movement
  (`|ExecutionSequence`
    (:`then_0`
      (set `self.DeltaSeconds` DeltaSeconds)
      (`self.K2_SetActorLocation` (+ (`self.K2_GetActorLocation`) (`KismetMathLibrary.MakeVector` (`self.VertSpeed`) (`self.HozSpeed`))) true)
      (`self.K2_SetActorRotation` (`KismetMathLibrary.RInterpTo_Constant` (`self.K2_GetActorRotation`) (`KismetMathLibrary.MakeRotator` (* (`self.HozSpeed`) 2.0)) (`self.DeltaSeconds`) 800.0)))
    (:`then_1`
      ;[1 1 1] Timer + min Score
      (`KismetSystemLibrary.Delay` 1.0)
      (if (== (`self.Seconds`) 0)
        (if (not (>= (`self.Score`) 0))
          (`/Game/Blueprints/GameMode_BP.GameOver` (`self.BP_GameMode`))
          (`GameplayStatics.PlaySound2D` "/Game/Soundtracks/Tiros/435201__mattix__game-over-01-voices.435201__mattix__game-over-01-voices" 1.0 1.0 0.0 null null))
        (else
          (set `self.Seconds` (- (`self.Seconds`) 1)))))))

(event `InputAxis|Mover_Cima_Embaixo`
  (params (AxisValue :type "Float (single-precision)"))
  ;[0.04042 1 0] Player input
  (bind _returndirectionspeed (`self.Movement` (`self.VertSpeed`) AxisValue))
  (set `self.VertSpeed` _returndirectionspeed))

(event `self.ReceiveAnyDamage`
  (params (Damage :type "Float (single-precision)") (DamageType :type "DamageType Object Reference") (InstigatedBy :type "Controller Object Reference") (DamageCauser :type "Actor Object Reference"))
  ;[1 1 1] Receber o Dano
  (if (`self.Invencivel`)
    (`GameplayStatics.PlaySound2D` "/Game/Soundtracks/Tiros/A_Test_Shield_01.A_Test_Shield_01" 1.0 1.0 0.0 null null)
    (else
      (set `self.Health` (- (`self.Health`) Damage))
      (set `self.Invencivel` true)
      (`GameplayStatics.PlaySound2D` "/Game/Soundtracks/Tiros/mixkit-cartoon-blow-impact-2654.mixkit-cartoon-blow-impact-2654" 1.0 1.0 0.0 null null)
      (if (<= (`self.Health`) 0.0)
        ;[1 1 1] Check health
        (`GameplayStatics.SpawnEmitterAtLocation` "/Game/Particle/P_BossExplosion.P_BossExplosion" (`self.K2_GetActorLocation`))
        (`/Game/Blueprints/GameMode_BP.GameOver` (`self.BP_GameMode`))
        (`GameplayStatics.PlaySound2D` "/Game/Soundtracks/Tiros/435201__mattix__game-over-01-voices.435201__mattix__game-over-01-voices" 1.0 1.0 0.0 null null)
        (else
          (`GameplayStatics.SpawnEmitterAttached` "/Game/Particle/Nave_Invicible/P_Ring.P_Ring" (`self.SkeletalMesh1`))
          (`KismetSystemLibrary.Delay` 3.0)
          (set `self.Invencivel` false))))))

(event `InputAxis|Mover`
  (params (AxisValue :type "Float (single-precision)"))
  ;[0.04042 1 0] Player input
  (bind _returndirectionspeed (`self.Movement` (`self.HozSpeed`) AxisValue))
  (set `self.HozSpeed` _returndirectionspeed))

(event `self.ReceiveHit`
  (params (MyComp :type "PrimitiveComponent Object Reference") (Other :type "Actor Object Reference") (OtherComp :type "PrimitiveComponent Object Reference") (bSelfMoved :type Boolean) (HitLocation :type "Vector Structure") (HitNormal :type "Vector Structure") (NormalImpulse :type "Vector Structure") (Hit :type "HitResult Structure (by ref)"))
  ;[1 1 1] Qnd Bate na parede volta com impulso.
  (set `self.VertSpeed` (* (* (`KismetMathLibrary.Abs` (`self.VertSpeed`)) 1.5) (.x HitNormal)))
  (set `self.HozSpeed` (* (* (`KismetMathLibrary.Abs` (`self.HozSpeed`)) 1.5) (.y HitNormal))))

(event `InputAction|Bomba`
  (params (Key :type "Key Structure"))
  ;[1 0.4786 0.4686] Player weaponry
  ;;[1 1 1] Nuke input
  (:`Pressed`
    (if (> (`self.Bomba`) 0)
      (`/Engine/EditorBlueprintResources/StandardMacros.DoOnce` false :!label _label
        (:`Completed`
          (`self.BombExplosion`)
          (`KismetSystemLibrary.Delay` 3.0)
          (goto _label :!via `Reset`))))))

(event `InputAxis|PrimaryFire`
  (params (AxisValue :type "Float (single-precision)"))
  ;[1 0.4786 0.4686] Player weaponry
  ;;[1 1 1] PrimaryFire
  (`/Engine/EditorBlueprintResources/StandardMacros.Gate` true :!label _label_2
    (:`Exit`
      (switch `int` (`self.PickupTypes`)
        (:`0`
          ;;[1 1 1] Default weapon
          (`/Engine/EditorBlueprintResources/StandardMacros.DoOnce` false :!label _label_3
            (:`Completed`
              (`self.PrimaryFire`)
              (`GameplayStatics.PlaySound2D` "/Game/Soundtracks/Tiros/Sound_2019_06_30_10_59_56_639__online-audio-converter_com_.Sound_2019_06_30_10_59_56_639__online-audio-converter_com_" 1.0 1.0 0.0 null null)
              (`KismetSystemLibrary.RetriggerableDelay` 0.3)
              (goto _label_3 :!via `Reset`))))
        (:`1`
          ;;[1 1 1] Machinegun
          (`/Engine/EditorBlueprintResources/StandardMacros.DoOnce` false :!label _label_4
            (:`Completed`
              (`self.MachineGun`)
              (`GameplayStatics.PlaySound2D` "/Game/Soundtracks/Tiros/Sound_2019_06_30_10_59_56_639__online-audio-converter_com_.Sound_2019_06_30_10_59_56_639__online-audio-converter_com_" 1.0 1.0 0.0 null null)
              (`KismetSystemLibrary.RetriggerableDelay` 0.15)
              (goto _label_4 :!via `Reset`))))
        (:`2`
          ;;[1 1 1] Multi-shot
          (`/Engine/EditorBlueprintResources/StandardMacros.DoOnce` false :!label _label_5
            (:`Completed`
              (`self.SpreadGun`)
              (`GameplayStatics.PlaySound2D` "/Game/Soundtracks/Tiros/Sound_2019_06_30_10_59_56_639__online-audio-converter_com_.Sound_2019_06_30_10_59_56_639__online-audio-converter_com_" 1.0 1.0 0.0 null null)
              (`KismetSystemLibrary.RetriggerableDelay` 0.3)
              (goto _label_5 :!via `Reset`))))))))

(event `InputAction|PrimaryFire`
  (params (Key :type "Key Structure"))
  ;[1 0.4786 0.4686] Player weaponry
  ;;[1 1 1] PrimaryFire
  (:`Pressed`
    (goto _label_2 :!via `Open`))
  (:`Released`
    (goto _label_2 :!via `Close`)))

(event `Key|Escape` :paused true
  (params (Key :type "Key Structure"))
  (bind _returnvalue (`GameplayStatics.GetPlayerController` 0))
  (:`Pressed`
    (`/Engine/EditorBlueprintResources/StandardMacros.FlipFlop`
      (:`A`
        (bind _returnvalue_2 (`|CreateWidget` "/Game/UI/WBP_PauseMenu.WBP_PauseMenu_C"))
        (`UserWidget.AddToViewport` _returnvalue_2 0)
        (`GameplayStatics.SetGamePaused` true)
        (set `PlayerController.bShowMouseCursor` true _returnvalue))
      (:`B`
        (`Widget.RemoveFromParent` _returnvalue_2)
        (`GameplayStatics.SetGamePaused` false)
        (set `PlayerController.bShowMouseCursor` false _returnvalue)))))

(fn `BombExplosion`
  (set `self.Bomba` (- (`self.Bomba`) 1))
  (`|SpawnActorFromClass` "/Game/PicksUps/Bomb/BP_Bomb.BP_Bomb_C" (`KismetMathLibrary.MakeTransform` (- (`self.K2_GetActorLocation`) (0.0 0.0 20.0)) (struct) (3.0 3.0 3.0)) "Undefined" "OverrideRootScale" null self))

(fn `MachineGun`
  (locals (ProjectileColour :type "LinearColor Structure" :default (struct)))
  (`|SpawnActorFromClass` "/Game/PlayerAirship/BP_Projectile_MachineGun.BP_Projectile_MachineGun_C" (`SceneComponent.K2_GetComponentToWorld` (`self.ProjectileSpawnMachineGun`)) "Undefined" "OverrideRootScale" null (`local.ProjectileColour`) self))

(fn `Movement`
  (params (Speed :type "Float (double-precision)") (Direction :type "Float (double-precision)"))
  (returns (ReturnDirectionSpeed :type "Float (double-precision)"))
  (return (`KismetMathLibrary.FInterpTo` Speed (* (`self.MovementSpeed`) Direction) (`self.DeltaSeconds`) 15.0)))

(fn `PrimaryFire`
  (locals (ProjectColour :type "LinearColor Structure" :default (struct :`G` 0.37942 :`B` 1.0)))
  (`|SpawnActorFromClass` "/Game/PlayerAirship/BP_Projectile_Default.BP_Projectile_Default_C" (`SceneComponent.K2_GetComponentToWorld` (`self.ProjectileSpawn`)) "AlwaysSpawn" "OverrideRootScale" null (`local.ProjectColour`) self))

(fn `SpreadGun`
  (locals (Colour :type "LinearColor Structure" :default (struct)))
  (bind _colour (`local.Colour`))
  (`|SpawnActorFromClass` "/Game/PlayerAirship/BP_Projectile_Spread.BP_Projectile_Spread_C" (`SceneComponent.K2_GetComponentToWorld` (`self.ProjectileSpread`)) "AlwaysSpawn" "OverrideRootScale" null _colour self)
  (`|SpawnActorFromClass` "/Game/PlayerAirship/BP_Projectile_Spread.BP_Projectile_Spread_C" (`SceneComponent.K2_GetComponentToWorld` (`self.ProjectileSpread02`)) "AlwaysSpawn" "OverrideRootScale" null _colour self)
  (`|SpawnActorFromClass` "/Game/PlayerAirship/BP_Projectile_Spread.BP_Projectile_Spread_C" (`SceneComponent.K2_GetComponentToWorld` (`self.ProjectileSpread03`)) "AlwaysSpawn" "OverrideRootScale" null _colour self))

(fn `UserConstructionScript`
  (set `self.Health` (`self.MaxHealth`)))