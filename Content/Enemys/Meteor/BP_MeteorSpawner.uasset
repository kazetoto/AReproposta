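; Meteor spawner that continuously feeds meteors into the level after a short startup delay.
; BeginPlay runs an endless delay loop that calls SpawnMeteoro, then waits MeteorFreq before the next spawn.
; Each spawn cycles through three meteor classes via MeteorSelection, at fixed X and Z with random Y.
; A random integer multiplier sets both the meteor's scale and its Resistencia, so bigger meteors get proportionally higher resistance.
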(event `self.ReceiveBeginPlay`
  (`KismetSystemLibrary.Delay` 0.2)
  (`KismetSystemLibrary.Delay` 1.0)
  (for _ (range 1) :!label _label
    (`self.SpawnMeteoro`)
    (`KismetSystemLibrary.Delay` (`self.MeteorFreq`))
    (goto _label)))

(fn `SpawnMeteoro`
  (bind _fixedrandomvalue (`self.FixedRandomValue`))
  (bind _returnvalue (`KismetMathLibrary.MakeVector` 2500.0 (`KismetMathLibrary.RandomFloatInRange` -900.0 900.0) 400.0))
  (bind _output_get (set `self.FixedRandomValue` (`KismetMathLibrary.RandomIntegerInRange` 1 3)))
  (switch `int` (`self.MeteorSelection`)
    (:`0`
      (bind _returnvalue_2 (* (1.0 1.0 1.0) _output_get))
      (bind _returnvalue_3 (`|SpawnActorFromClass` "/Game/Enemys/Meteor/BP_Meteor_01.BP_Meteor_01_C" (`KismetMathLibrary.MakeTransform` _returnvalue (struct) _returnvalue_2) "Undefined" "OverrideRootScale" null null))
      (set `/Game/Enemys/Meteor/BP_Meteor_01.Resistencia` (* _fixedrandomvalue (`/Game/Enemys/Meteor/BP_Meteor_01.Resistencia` _returnvalue_3)) _returnvalue_3)
      (bind _result (`/Engine/EditorBlueprintResources/StandardMacros.IncrementInt` (`self.MeteorSelection`) :!label _label)
        (:`  `
          (set `self.MeteorSelection` _result))))
    (:`1`
      (bind _returnvalue_4 (`|SpawnActorFromClass` "/Game/Enemys/Meteor/BP_Meteor_02.BP_Meteor_02_C" (`KismetMathLibrary.MakeTransform` _returnvalue (struct) _returnvalue_2) "Undefined" "OverrideRootScale" null null))
      (set `/Game/Enemys/Meteor/BP_Meteor_02.Resistencia` (* _fixedrandomvalue (`/Game/Enemys/Meteor/BP_Meteor_02.Resistencia` _returnvalue_4)) _returnvalue_4)
      (goto _label))
    (:`2`
      (bind _returnvalue_5 (`|SpawnActorFromClass` "/Game/Enemys/Meteor/BP_Meteor_03.BP_Meteor_03_C" (`KismetMathLibrary.MakeTransform` _returnvalue (struct) _returnvalue_2) "Undefined" "OverrideRootScale" null null))
      (set `/Game/Enemys/Meteor/BP_Meteor_03.Resistencia` (* _fixedrandomvalue (`/Game/Enemys/Meteor/BP_Meteor_03.Resistencia` _returnvalue_5)) _returnvalue_5)
      (set `self.MeteorSelection` 0))))

(fn `UserConstructionScript`)