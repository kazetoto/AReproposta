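; BP_Meteor_02 is a meteor enemy that can be shot down or crash into the player ship.
; Incoming damage lowers its Resistencia value, and the actor is destroyed when that reaches zero or below.
; When its capsule overlaps a BP_Nave_Proposta2, it applies fixed damage to the ship, spawns an explosion particle at its location and destroys itself.
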(event `self.ReceiveAnyDamage`
  (params (Damage :type "Float (single-precision)") (DamageType :type "DamageType Object Reference") (InstigatedBy :type "Controller Object Reference") (DamageCauser :type "Actor Object Reference"))
  (bind _output_get (set `self.Resistencia` (- (`self.Resistencia`) Damage)))
  (if (<= _output_get 0.0)
    (`self.K2_DestroyActor` :!label _label)))

(event `self.Capsule.OnComponentBeginOverlap`
  (params (OverlappedComponent :type "PrimitiveComponent Object Reference") (OtherActor :type "Actor Object Reference") (OtherComp :type "PrimitiveComponent Object Reference") (OtherBodyIndex :type Integer) (bFromSweep :type Boolean) (SweepResult :type "HitResult Structure (by ref)"))
  (bind _asbp_nave_proposta_2 (cast `/Game/NAVE_PROPOSTA/BP_Nave_Proposta2` OtherActor))
  (`GameplayStatics.ApplyDamage` _asbp_nave_proposta_2 10.0 null self)
  (`GameplayStatics.SpawnEmitterAtLocation` "/Game/StarterContent/Particles/P_Explosion.P_Explosion" (`self.K2_GetActorLocation` self))
  (goto _label))

(fn `UserConstructionScript`)