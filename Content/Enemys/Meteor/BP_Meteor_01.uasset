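; BP_Meteor_01 is a destructible meteor enemy that hurts the player airship on contact and drops a weapon pickup when shot down.
; Incoming damage lowers Resistencia; at zero it plays a sound, spawns a random bomb, machine gun or spread pickup, then explodes and destroys itself.
; Capsule overlap with BP_PlayerAirship applies fixed damage and destroys the meteor with a smaller explosion and no drop.
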(event `self.ReceiveAnyDamage`
  (params (Damage :type "Float (single-precision)") (DamageType :type "DamageType Object Reference") (InstigatedBy :type "Controller Object Reference") (DamageCauser :type "Actor Object Reference"))
  (bind _returnvalue (`self.K2_GetActorLocation` self))
  (bind _output_get (set `self.Resistencia` (- (`self.Resistencia`) Damage)))
  (if (<= _output_get 0.0)
    (`GameplayStatics.PlaySound2D` "/Game/Soundtracks/Tiros/A_Test_Shield_02.A_Test_Shield_02" 1.0 1.0 0.0 null null)
    (switch `int` (`KismetMathLibrary.RandomIntegerInRange` 0 2)
      (:`0`
        (`|SpawnActorFromClass` "/Game/PicksUps/Bomb/BP_BombPickup.BP_BombPickup_C" (`KismetMathLibrary.MakeTransform` _returnvalue) "Undefined" "OverrideRootScale" null null))
      (:`1`
        (`|SpawnActorFromClass` "/Game/PicksUps/MachineGun/BP_MachineGunPickup.BP_MachineGunPickup_C" (`KismetMathLibrary.MakeTransform` _returnvalue) "Undefined" "OverrideRootScale" null null))
      (:`2`
        (`|SpawnActorFromClass` "/Game/PicksUps/SpreadGun/BP_SpreadPickup.BP_SpreadPickup_C" (`KismetMathLibrary.MakeTransform` _returnvalue) "Undefined" "OverrideRootScale" null null)))
    (`GameplayStatics.SpawnEmitterAtLocation` "/Game/StarterContent/Particles/P_Explosion.P_Explosion" _returnvalue (struct) (2.0 2.0 2.0))
    (`self.K2_DestroyActor` self)))

(event `self.Capsule.OnComponentBeginOverlap`
  (params (OverlappedComponent :type "PrimitiveComponent Object Reference") (OtherActor :type "Actor Object Reference") (OtherComp :type "PrimitiveComponent Object Reference") (OtherBodyIndex :type Integer) (bFromSweep :type Boolean) (SweepResult :type "HitResult Structure (by ref)"))
  (bind _asbp_player_airship (cast `/Game/PlayerAirship/BP_PlayerAirship` OtherActor))
  (`GameplayStatics.ApplyDamage` _asbp_player_airship 10.0 null self)
  (`GameplayStatics.SpawnEmitterAtLocation` "/Game/StarterContent/Particles/P_Explosion.P_Explosion" (`self.K2_GetActorLocation` self))
  (`self.K2_DestroyActor`))

(fn `UserConstructionScript`)