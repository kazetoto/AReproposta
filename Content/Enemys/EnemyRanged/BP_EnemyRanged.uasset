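; Ranged enemy ship that fights the player's BP_Nave_Proposta2 ship with twin projectiles.
; A Timeline glides it to its spawn position with box collision off, then enables collision and movement.
; Tick drifts it along negative X while bouncing between Y limits, and a looping Delay fires from two arrows.
; Lethal damage explodes it and awards score; ramming the player deals damage and destroys it.
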(event `self.ReceiveBeginPlay`
  (bind _box (`self.Box`))
  (bind _asbp_nave_proposta_2 (cast `/Game/NAVE_PROPOSTA/BP_Nave_Proposta2` (`GameplayStatics.GetPlayerPawn` 0)))
  (set `self.Player` _asbp_nave_proposta_2)
  (`PrimitiveComponent.SetCollisionEnabled` _box "NoCollision")
  (bind (_direction _newtrack_0) (`Timeline|Timeline_0`)
    (:`Update`
      (`self.K2_SetActorLocation` (`KismetMathLibrary.VLerp` (`self.K2_GetActorLocation`) (`KismetMathLibrary.MakeVector` (`self.Spawn`) 0.0 400.0) (* _newtrack_0 (`GameplayStatics.GetWorldDeltaSeconds`))) true))
    (:`Finished`
      (`PrimitiveComponent.SetCollisionEnabled` _box "QueryOnly")
      (set `self.CanMove` true))))

(event `self.ReceiveTick`
  (params (DeltaSeconds :type "Float (single-precision)"))
  (bind (_returnvalue_x _returnvalue_y) (`KismetMathLibrary.BreakVector` (`self.K2_GetActorLocation`)))
  (bind _arrow (`self.Arrow`))
  (bind _arrow1 (`self.Arrow1`))
  (if (`self.CanMove`)
    (`self.K2_SetActorLocation` (+ (`self.K2_GetActorLocation`) (+ (`KismetMathLibrary.MakeVector` -1.2 (* (`self.Speed`) (`KismetMathLibrary.SelectFloat` -1.0 1.0 (`self.Left`)))) DeltaSeconds)))
    (if (<= _returnvalue_y -750.0)
      (set `self.Left` false)
      (elif (>= _returnvalue_y 750.0)
        (set `self.Left` true)))
    ;[1 1 1] Atirando
    (`KismetSystemLibrary.Delay` 2.0 :!label _label)
    (`|SpawnActorFromClass` "/Game/Enemys/EnemyRanged/BP_EnemyRanged_Projectile.BP_EnemyRanged_Projectile_C" (`KismetMathLibrary.MakeTransform` (`SceneComponent.K2_GetComponentLocation` _arrow) (`SceneComponent.K2_GetComponentRotation` _arrow)) "Undefined" "OverrideRootScale" null null)
    (`|SpawnActorFromClass` "/Game/Enemys/EnemyRanged/BP_EnemyRanged_Projectile.BP_EnemyRanged_Projectile_C" (`KismetMathLibrary.MakeTransform` (`SceneComponent.K2_GetComponentLocation` _arrow1) (`SceneComponent.K2_GetComponentRotation` _arrow1)) "Undefined" "OverrideRootScale" null null)
    (goto _label)))

(event `self.ReceiveAnyDamage`
  (params (Damage :type "Float (single-precision)") (DamageType :type "DamageType Object Reference") (InstigatedBy :type "Controller Object Reference") (DamageCauser :type "Actor Object Reference"))
  (bind _player (`self.Player`))
  ;[1 1 1] Vida do Ranger
  (bind _output_get (set `self.Vida_Enemy` (- (`self.Vida_Enemy`) Damage)))
  (if (<= _output_get 0.0)
    (`GameplayStatics.SpawnEmitterAtLocation` "/Game/Particle/Sparks_With_Explosions.Sparks_With_Explosions" (`self.K2_GetActorLocation`) (struct) (2.0 2.0 2.0))
    (set `/Game/NAVE_PROPOSTA/BP_Nave_Proposta2.Score` (+ (`/Game/NAVE_PROPOSTA/BP_Nave_Proposta2.Score` _player) 50) _player)
    (`self.K2_DestroyActor` :!label _label_2)))

(event `self.Box.OnComponentBeginOverlap`
  (params (OverlappedComponent :type "PrimitiveComponent Object Reference") (OtherActor :type "Actor Object Reference") (OtherComp :type "PrimitiveComponent Object Reference") (OtherBodyIndex :type Integer) (bFromSweep :type Boolean) (SweepResult :type "HitResult Structure (by ref)"))
  (bind _asbp_nave_proposta_2 (cast `/Game/NAVE_PROPOSTA/BP_Nave_Proposta2` OtherActor))
  (`GameplayStatics.ApplyDamage` _asbp_nave_proposta_2 10.0)
  (`GameplayStatics.SpawnEmitterAtLocation` "/Game/Particle/Sparks_With_Explosions.Sparks_With_Explosions" (`self.K2_GetActorLocation`))
  (goto _label_2))

(fn `UserConstructionScript`)