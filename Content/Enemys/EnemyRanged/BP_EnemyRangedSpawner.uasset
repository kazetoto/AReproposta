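; Spawner that produces waves of ranged enemies (BP_EnemyRanged) for as long as it runs.
; After a short startup pause and a configurable initial delay, BeginPlay spawns a batch sized by EnemyRangedQuant, then repeats every EnemyRangedFreq seconds.
; SpawnEnemies places each enemy at fixed world X and height with random Y, then randomizes its Speed, Left flag and Spawn value.
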(event `self.ReceiveBeginPlay`
  (`KismetSystemLibrary.Delay` 0.2)
  (`KismetSystemLibrary.Delay` (`self.EnemyRangedSpawnDelay`))
  (for _ (range (+ (`self.EnemyRangedQuant`) 1)) :!label _label
    (`self.SpawnEnemies`))
  (`KismetSystemLibrary.Delay` (`self.EnemyRangedFreq`))
  (goto _label))

(fn `SpawnEnemies`
  (bind _returnvalue (`|SpawnActorFromClass` "/Game/Enemys/EnemyRanged/BP_EnemyRanged.BP_EnemyRanged_C" (`KismetMathLibrary.MakeTransform` (`KismetMathLibrary.MakeVector` 2000.0 (`KismetMathLibrary.RandomFloatInRange` -750.0 750.0) 400.0)) "Undefined" "OverrideRootScale" null null))
  (set `/Game/Enemys/EnemyRanged/BP_EnemyRanged.Speed` (`KismetMathLibrary.RandomFloatInRange` 5.0 10.0) _returnvalue)
  (set `/Game/Enemys/EnemyRanged/BP_EnemyRanged.Left` (`KismetMathLibrary.RandomBool`) _returnvalue)
  (set `/Game/Enemys/EnemyRanged/BP_EnemyRanged.Spawn` (`KismetMathLibrary.RandomFloatInRange` 1000.0 2000.0) _returnvalue))

(fn `UserConstructionScript`)