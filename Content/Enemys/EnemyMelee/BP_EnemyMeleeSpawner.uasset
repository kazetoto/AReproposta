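; BP_EnemyMeleeSpawner spawns recurring waves of BP_EnemyMelee enemies for as long as it is in play.
; After an initial delay, BeginPlay loops forever, calling SpawnMelee for each enemy in the wave, then waiting for the wave interval.
; SpawnMelee places each enemy at hard-coded world X and Z with random Y, independent of the spawner's location, then randomizes its Speed, Foward flag and Spawn value.
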(event `self.ReceiveBeginPlay`
  (`KismetSystemLibrary.Delay` 0.2)
  (`KismetSystemLibrary.Delay` (`self.EnemyMeleSpawnDelay`))
  (for _ (range (+ (`self.EnemyMeleQuant`) 1)) :!label _label
    (`self.Spawn_Melee`))
  (`KismetSystemLibrary.Delay` (`self.EnemyMeleFreq`))
  (goto _label))

(fn `Spawn_Melee`
  (bind _returnvalue (`|SpawnActorFromClass` "/Game/Enemys/EnemyMelee/BP_EnemyMelee.BP_EnemyMelee_C" (`KismetMathLibrary.MakeTransform` (`KismetMathLibrary.MakeVector` 2000.0 (`KismetMathLibrary.RandomFloatInRange` -750.0 750.0) 400.0)) "Undefined" "OverrideRootScale" null null))
  (set `/Game/Enemys/EnemyMelee/BP_EnemyMelee.Speed` (`KismetMathLibrary.RandomFloatInRange` 5.0 10.0) _returnvalue)
  (set `/Game/Enemys/EnemyMelee/BP_EnemyMelee.Foward` (`KismetMathLibrary.RandomBool`) _returnvalue)
  (set `/Game/Enemys/EnemyMelee/BP_EnemyMelee.Spawn` (`KismetMathLibrary.RandomFloatInRange` 1000.0 1700.0) _returnvalue))

(fn `UserConstructionScript`)