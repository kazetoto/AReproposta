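; Melee enemy that attacks the player airship by ramming it and awards score when shot down.
; On spawn a timeline lerps it into position with collision off, then enables collision and movement.
; Tick drifts it along negative X at random rates while bouncing between Y limits, with frame-rate-dependent steps.
; Lethal damage adds score and plays a sound; ramming damages the player, and both paths explode and destroy it.
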(event `self.ReceiveBeginPlay`
  (bind _capsule (`self.Capsule`))
  (bind _asbp_player_airship (cast `/Game/PlayerAirship/BP_PlayerAirship` (`GameplayStatics.GetPlayerPawn` 0)))
  (set `self.Player` _asbp_player_airship)
  (`PrimitiveComponent.SetCollisionEnabled` _capsule "NoCollision")
  (bind (_direction _newtrack_0) (`Timeline|Timeline_0`)
    (:`Update`
      (`self.K2_SetActorLocation` (`KismetMathLibrary.VLerp` (`self.K2_GetActorLocation`) (`KismetMathLibrary.MakeVector` (`self.Spawn`) 0.0 400.0) (* _newtrack_0 (`GameplayStatics.GetWorldDeltaSeconds`))) true))
    (:`Finished`
      (`PrimitiveComponent.SetCollisionEnabled` _capsule "QueryOnly")
      (set `self.CanMove` true))))

(event `self.ReceiveTick`
  (params (DeltaSeconds :type "Float (single-precision)"))
  (bind (_returnvalue_x _returnvalue_y) (`KismetMathLibrary.BreakVector` (`self.K2_GetActorLocation`)))
  ;[1 1 1] Foward/Backwards movement
  (if (`self.CanMove`)
    (`self.K2_SetActorLocation` (+ (`self.K2_GetActorLocation`) (+ (`KismetMathLibrary.MakeVector` (`KismetMathLibrary.RandomFloatInRange` -2.0 -8.0) (* (`self.Speed`) (`KismetMathLibrary.SelectFloat` -1.0 1.0 (`self.Foward`)))) DeltaSeconds)) true)
    (if (<= _returnvalue_y -800.0)
      (set `self.Foward` false)
      (elif (>= _returnvalue_y 800.0)
        (set `self.Foward` true)))))

(event `self.ReceiveAnyDamage`
  (params (Damage :type "Float (single-precision)") (DamageType :type "DamageType Object Reference") (InstigatedBy :type "Controller Object Reference") (DamageCauser :type "Actor Object Reference"))
  (bind _player (`self.Player`))
  ;[1 1 1] Vida do Melee
  (bind _output_get (set `self.Vida_Enemy` (- (`self.Vida_Enemy`) Damage)))
  (if (<= _output_get 0.0)
    (set `/Game/PlayerAirship/BP_PlayerAirship.Score` (+ (`/Game/PlayerAirship/BP_PlayerAirship.Score` _player) 150) _player)
    (`GameplayStatics.PlaySound2D` "/Game/Soundtracks/Tiros/A_Test_Impact_03.A_Test_Impact_03" 1.0 1.0 0.0 null null)
    (`GameplayStatics.SpawnEmitterAtLocation` "/Game/Particle/P_Sparks_With_Explosions.P_Sparks_With_Explosions" (`self.K2_GetActorLocation`) (struct) (2.0 2.0 2.0) :!label _label)
    (`self.K2_DestroyActor`)))

(event `self.Capsule.OnComponentBeginOverlap`
  (params (OverlappedComponent :type "PrimitiveComponent Object Reference") (OtherActor :type "Actor Object Reference") (OtherComp :type "PrimitiveComponent Object Reference") (OtherBodyIndex :type Integer) (bFromSweep :type Boolean) (SweepResult :type "HitResult Structure (by ref)"))
  ;[1 1 1] Vida do Melee
  (bind _asbp_player_airship (cast `/Game/PlayerAirship/BP_PlayerAirship` OtherActor))
  (`GameplayStatics.ApplyDamage` _asbp_player_airship 10.0)
  (goto _label))

(fn `UserConstructionScript`)