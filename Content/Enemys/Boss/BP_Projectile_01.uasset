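; Boss enemy projectile that damages the player's airship and can itself be shot down.
; A capsule overlap with BP_PlayerAirship applies fixed damage, spawns an explosion and destroys the projectile.
; Incoming damage reduces the projectile's own HP, and at zero it explodes and is destroyed.
; On BeginPlay a short delay starts, after which the projectile destroys itself if it has hit nothing.
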(event `self.ReceiveAnyDamage`
  (params (Damage :type "Float (single-precision)") (DamageType :type "DamageType Object Reference") (InstigatedBy :type "Controller Object Reference") (DamageCauser :type "Actor Object Reference"))
  ;[1 1 1] Vida do projetil
  (set `self.BProjectileHP` (`KismetMathLibrary.FClamp` (- (`self.BProjectileHP`) Damage) 0.0 (`self.BProjectileHP`)))
  (if (<= (`self.BProjectileHP`) 0.0)
    (`GameplayStatics.SpawnEmitterAtLocation` "/Game/StarterContent/Particles/P_Explosion.P_Explosion" (`self.K2_GetActorLocation` self))
    (`self.K2_DestroyActor`)))

(event `self.Capsule.OnComponentBeginOverlap`
  (params (OverlappedComponent :type "PrimitiveComponent Object Reference") (OtherActor :type "Actor Object Reference") (OtherComp :type "PrimitiveComponent Object Reference") (OtherBodyIndex :type Integer) (bFromSweep :type Boolean) (SweepResult :type "HitResult Structure (by ref)"))
  ;[1 1 1] Aplicar dano somente em player
  (bind _asbp_player_airship (cast `/Game/PlayerAirship/BP_PlayerAirship` OtherActor))
  (`GameplayStatics.ApplyDamage` _asbp_player_airship 10.0 null self)
  (`GameplayStatics.SpawnEmitterAtLocation` "/Game/StarterContent/Particles/P_Explosion.P_Explosion" (`self.K2_GetActorLocation`) (struct) (1.0 1.0 1.0) false)
  (`self.K2_DestroyActor` self)
  (`KismetSystemLibrary.PrintString` "Player Hited"))

(event `self.ReceiveBeginPlay`
  ;[1 1 1] Desaparecer caso nao acerte nada
  (`KismetSystemLibrary.Delay` 3.0)
  (`self.K2_DestroyActor`))

(fn `UserConstructionScript`)