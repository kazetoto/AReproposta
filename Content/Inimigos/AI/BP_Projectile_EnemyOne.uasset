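; BP_Projectile_EnemyOne is an enemy projectile that damages whatever its static mesh overlaps.
; The mesh's begin-overlap event applies the Damage variable to the other actor, spawns a sparks-and-explosion emitter at the projectile's location, destroys the projectile and prints a debug hit message.
; There is no filter on what it hits, and the component hit event is empty.
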(event `self.StaticMesh.OnComponentBeginOverlap`
  (params (OverlappedComponent :type "PrimitiveComponent Object Reference") (OtherActor :type "Actor Object Reference") (OtherComp :type "PrimitiveComponent Object Reference") (OtherBodyIndex :type Integer) (bFromSweep :type Boolean) (SweepResult :type "HitResult Structure (by ref)"))
  (`GameplayStatics.ApplyDamage` OtherActor (`self.Damage`))
  (`GameplayStatics.SpawnEmitterAtLocation` "/Game/Particle/Sparks_With_Explosions.Sparks_With_Explosions" (`self.K2_GetActorLocation`) (struct) (1.0 1.0 1.0) false)
  (`self.K2_DestroyActor` self)
  (`KismetSystemLibrary.PrintString` "Enemy hit you"))

(event `self.StaticMesh.OnComponentHit`
  (params (HitComponent :type "PrimitiveComponent Object Reference") (OtherActor :type "Actor Object Reference") (OtherComp :type "PrimitiveComponent Object Reference") (NormalImpulse :type "Vector Structure") (Hit :type "HitResult Structure (by ref)")))

(fn `UserConstructionScript`
  (`parent.UserConstructionScript`))