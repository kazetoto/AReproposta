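; Test spawner that creates a ranged pickup enemy (Enemy_Teste_Range_Pickup) 15 seconds after BeginPlay.
; A DoOnce and single-iteration loop call SpawnEnemiesPickups, then delays lead to resetting the gate, though nothing re-enters it, so only one spawn occurs.
; The spawn function uses a fixed position, then sets the enemy's speed, random left flag and random SpawnPickup value.
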(event `self.ReceiveBeginPlay`
  (`KismetSystemLibrary.Delay` 15.0)
  (`/Engine/EditorBlueprintResources/StandardMacros.DoOnce` false :!label _label
    (:`Completed`
      (for _ (range 1)
        (`self.SpawnEnemiesPickups`)
        ;[1 1 1] Tempo de Spawn
        (`KismetSystemLibrary.Delay` 60.0)
        (`KismetSystemLibrary.Delay` 10.0)
        (goto _label :!via `Reset`)))))

(fn `SpawnEnemiesPickups`
  (bind _returnvalue (`|SpawnActorFromClass` "/Game/Inimigos/AI/Teste(Ranger)/Enemy_Teste_Range_Pickup.Enemy_Teste_Range_Pickup_C" (`KismetMathLibrary.MakeTransform` (`KismetMathLibrary.MakeVector` 2900.0 60.0 (`KismetMathLibrary.RandomFloatInRange` 430.0 430.0))) "Undefined" "OverrideRootScale" null null))
  (set `/Game/Inimigos/AI/Teste(Ranger)/Enemy_Teste_Range_Pickup.SpeedPickup` (`KismetMathLibrary.RandomFloatInRange` 10.0 10.0) _returnvalue)
  (set `/Game/Inimigos/AI/Teste(Ranger)/Enemy_Teste_Range_Pickup.LeftPickup` (`KismetMathLibrary.RandomBool`) _returnvalue)
  (set `/Game/Inimigos/AI/Teste(Ranger)/Enemy_Teste_Range_Pickup.SpawnPickup` (`KismetMathLibrary.RandomFloatInRange` 500.0 -1000.0) _returnvalue))

(fn `UserConstructionScript`)