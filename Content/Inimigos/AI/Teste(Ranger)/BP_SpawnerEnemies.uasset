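; Spawner actor for a test ranged enemy (Enemy_Teste_Range02) that creates a batch of them when play begins.
; A BeginPlay loop calls SpawnEnemies, which places each enemy at the same fixed point and randomizes its Speed, Left flag and Spawn value.
; The Delay inside the loop does not stagger spawns, so the whole batch appears at once and the spawner destroys itself after the delay.
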(event `self.ReceiveBeginPlay`
  (for _ (range 6)
    (`self.SpawnEnemies`)
    ;[1 1 1] Tempo de Spawn
    (`KismetSystemLibrary.Delay` 120.0)
    (`self.K2_DestroyActor`)))

(fn `SpawnEnemies`
  (bind _returnvalue (`|SpawnActorFromClass` "/Game/Inimigos/AI/Teste(Ranger)/Enemy_Teste_Range02.Enemy_Teste_Range02_C" (`KismetMathLibrary.MakeTransform` (`KismetMathLibrary.MakeVector` 3000.0 -900.0 (`KismetMathLibrary.RandomFloatInRange` 430.0 430.0))) "Undefined" "OverrideRootScale" null null))
  (set `/Game/Inimigos/AI/Teste(Ranger)/Enemy_Teste_Range02.Speed` (`KismetMathLibrary.RandomFloatInRange` -10.0 20.0) _returnvalue)
  (set `/Game/Inimigos/AI/Teste(Ranger)/Enemy_Teste_Range02.Left` (`KismetMathLibrary.RandomBool`) _returnvalue)
  (set `/Game/Inimigos/AI/Teste(Ranger)/Enemy_Teste_Range02.Spawn` (`KismetMathLibrary.RandomFloatInRange` 500.0 -1500.0) _returnvalue))

(fn `UserConstructionScript`)