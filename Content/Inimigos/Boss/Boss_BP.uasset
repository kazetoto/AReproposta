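; Boss enemy that loses HP on any damage and, at zero, spawns a large explosion and destroys itself.
; When not attacking, Tick waits through a Delay, then randomly picks one of three attack events, with one roll left idle.
; The attacks fire staggered projectile pairs from arrow components, simultaneous Y-offset volleys, or two heavier-pattern BP_Projectile02 shots telegraphed by ring emitters.
; IsAttaking gates selection during each pattern.
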(event `self.ReceiveAnyDamage`
  (params (Damage :type "Float (single-precision)") (DamageType :type "DamageType Object Reference") (InstigatedBy :type "Controller Object Reference") (DamageCauser :type "Actor Object Reference"))
  (bind (_returnvalue_x _returnvalue_y _returnvalue_z) (`KismetMathLibrary.BreakVector` (`SceneComponent.K2_GetComponentLocation` (`self.BossHeadlow4`))))
  ;[1 1 1] Receber Dano Boss
  (set `self.BossHP` (- (`self.BossHP`) Damage))
  (`KismetSystemLibrary.PrintString` "Boss damaged")
  (if (<= (`self.BossHP`) 0.0)
    (`/Engine/EditorBlueprintResources/StandardMacros.DoOnce` false
      (:`Completed`
        (`GameplayStatics.SpawnEmitterAtLocation` "/Game/Particle/Explosion_Boss_Dead.Explosion_Boss_Dead" (`KismetMathLibrary.MakeVector` _returnvalue_x (+ _returnvalue_y 50.0) _returnvalue_z) (struct) (10.0 10.0 10.0))
        (`KismetSystemLibrary.Delay` 0.2)
        (`self.K2_DestroyActor`)))))

(event `PAtaque1`
  (bind _arrow8 (`self.Arrow8`))
  (bind _arrow1 (`self.Arrow1`))
  (bind _arrow5 (`self.Arrow5`))
  (bind _arrow2 (`self.Arrow2`))
  (bind _arrow6 (`self.Arrow6`))
  (bind _arrow3 (`self.Arrow3`))
  (bind _arrow7 (`self.Arrow7`))
  (bind _arrow4 (`self.Arrow4`))
  ;[1 1 1] Padrao de ataque 01/03
  (set `self.IsAttaking?` true)
  (`KismetSystemLibrary.Delay` 2.0)
  (`/Engine/EditorBlueprintResources/StandardMacros.DoOnce` false :!label _label
    (:`Completed`
      (`|SpawnActorFromClass` "/Game/Inimigos/Boss/BossProjectiles/BP_Projectile01.BP_Projectile01_C" (`KismetMathLibrary.MakeTransform` (`SceneComponent.K2_GetComponentLocation` _arrow1) (`SceneComponent.K2_GetComponentRotation` _arrow1)) "Undefined" "OverrideRootScale" null null)
      (`|SpawnActorFromClass` "/Game/Inimigos/Boss/BossProjectiles/BP_Projectile01.BP_Projectile01_C" (`KismetMathLibrary.MakeTransform` (`SceneComponent.K2_GetComponentLocation` _arrow5) (`SceneComponent.K2_GetComponentRotation` _arrow5)) "Undefined" "OverrideRootScale" null null)
      (`KismetSystemLibrary.Delay` 0.1)
      (`|SpawnActorFromClass` "/Game/Inimigos/Boss/BossProjectiles/BP_Projectile01.BP_Projectile01_C" (`KismetMathLibrary.MakeTransform` (`SceneComponent.K2_GetComponentLocation` _arrow2) (`SceneComponent.K2_GetComponentRotation` _arrow2)) "Undefined" "OverrideRootScale" null null)
      (`|SpawnActorFromClass` "/Game/Inimigos/Boss/BossProjectiles/BP_Projectile01.BP_Projectile01_C" (`KismetMathLibrary.MakeTransform` (`SceneComponent.K2_GetComponentLocation` _arrow6) (`SceneComponent.K2_GetComponentRotation` _arrow6)) "Undefined" "OverrideRootScale" null null)
      (`KismetSystemLibrary.Delay` 0.1)
      (`|SpawnActorFromClass` "/Game/Inimigos/Boss/BossProjectiles/BP_Projectile01.BP_Projectile01_C" (`KismetMathLibrary.MakeTransform` (`SceneComponent.K2_GetComponentLocation` _arrow3) (`SceneComponent.K2_GetComponentRotation` _arrow3)) "Undefined" "OverrideRootScale" null null)
      (`|SpawnActorFromClass` "/Game/Inimigos/Boss/BossProjectiles/BP_Projectile01.BP_Projectile01_C" (`KismetMathLibrary.MakeTransform` (`SceneComponent.K2_GetComponentLocation` _arrow7) (`SceneComponent.K2_GetComponentRotation` _arrow7)) "Undefined" "OverrideRootScale" null null)
      (`KismetSystemLibrary.Delay` 0.1)
      (`|SpawnActorFromClass` "/Game/Inimigos/Boss/BossProjectiles/BP_Projectile01.BP_Projectile01_C" (`KismetMathLibrary.MakeTransform` (`SceneComponent.K2_GetComponentLocation` _arrow4) (`SceneComponent.K2_GetComponentRotation` _arrow4)) "Undefined" "OverrideRootScale" null null)
      (`|SpawnActorFromClass` "/Game/Inimigos/Boss/BossProjectiles/BP_Projectile01.BP_Projectile01_C" (`KismetMathLibrary.MakeTransform` (`SceneComponent.K2_GetComponentLocation` _arrow8) (`SceneComponent.K2_GetComponentRotation` _arrow8)) "Undefined" "OverrideRootScale" null null)
      (`KismetSystemLibrary.Delay` 1.0)
      (set `self.IsAttaking?` false)
      (goto _label :!via `Reset`))))

(event `PAtaque2`
  (bind _arrow5 (`self.Arrow5`))
  (bind _arrow1 (`self.Arrow1`))
  (bind (_returnvalue_x _returnvalue_y _returnvalue_z) (`KismetMathLibrary.BreakVector` (`SceneComponent.K2_GetComponentLocation` _arrow5)))
  (bind _returnvalue (`SceneComponent.K2_GetComponentRotation` _arrow1))
  (bind _returnvalue_2 (`SceneComponent.K2_GetComponentRotation` _arrow5))
  (bind (_returnvalue_x_2 _returnvalue_y_2 _returnvalue_z_2) (`KismetMathLibrary.BreakVector` (`SceneComponent.K2_GetComponentLocation` _arrow1)))
  (bind _returnvalue_3 (- _returnvalue_y_2 200.0))
  (bind _returnvalue_4 (+ _returnvalue_y 200.0))
  ;[1 1 1] Padrao de ataque 2/3
  (set `self.IsAttaking?` true)
  (`KismetSystemLibrary.Delay` 2.0)
  (`|SpawnActorFromClass` "/Game/Inimigos/Boss/BossProjectiles/BP_Projectile01.BP_Projectile01_C" (`KismetMathLibrary.MakeTransform` (`KismetMathLibrary.MakeVector` _returnvalue_x_2 _returnvalue_y_2 _returnvalue_z_2) _returnvalue) "Undefined" "OverrideRootScale" null null)
  (`|SpawnActorFromClass` "/Game/Inimigos/Boss/BossProjectiles/BP_Projectile01.BP_Projectile01_C" (`KismetMathLibrary.MakeTransform` (`KismetMathLibrary.MakeVector` _returnvalue_x _returnvalue_y _returnvalue_z) _returnvalue_2) "Undefined" "OverrideRootScale" null null)
  (`|SpawnActorFromClass` "/Game/Inimigos/Boss/BossProjectiles/BP_Projectile01.BP_Projectile01_C" (`KismetMathLibrary.MakeTransform` (`KismetMathLibrary.MakeVector` _returnvalue_x_2 _returnvalue_3 _returnvalue_z_2) _returnvalue) "Undefined" "OverrideRootScale" null null)
  (`|SpawnActorFromClass` "/Game/Inimigos/Boss/BossProjectiles/BP_Projectile01.BP_Projectile01_C" (`KismetMathLibrary.MakeTransform` (`KismetMathLibrary.MakeVector` _returnvalue_x _returnvalue_4 _returnvalue_z) _returnvalue_2) "Undefined" "OverrideRootScale" null null)
  (`|SpawnActorFromClass` "/Game/Inimigos/Boss/BossProjectiles/BP_Projectile01.BP_Projectile01_C" (`KismetMathLibrary.MakeTransform` (`KismetMathLibrary.MakeVector` _returnvalue_x_2 (- _returnvalue_3 200.0) _returnvalue_z_2) _returnvalue) "Undefined" "OverrideRootScale" null null)
  (`|SpawnActorFromClass` "/Game/Inimigos/Boss/BossProjectiles/BP_Projectile01.BP_Projectile01_C" (`KismetMathLibrary.MakeTransform` (`KismetMathLibrary.MakeVector` _returnvalue_x (+ _returnvalue_4 200.0) _returnvalue_z) _returnvalue_2) "Undefined" "OverrideRootScale" null null)
  (set `self.IsAttaking?` false))

(event `PAtaque3`
  (bind _arrow (`self.Arrow`))
  (bind (_returnvalue_x _returnvalue_y _returnvalue_z) (`KismetMathLibrary.BreakVector` (`SceneComponent.K2_GetComponentLocation` _arrow)))
  (bind _returnvalue (`SceneComponent.K2_GetComponentRotation` _arrow))
  (bind _returnvalue_2 (- _returnvalue_y 600.0))
  (bind _returnvalue_3 (+ _returnvalue_y 600.0))
  ;[1 1 1] Padrao de ataque 03/03
  (set `self.IsAttaking?` true)
  (bind _returnvalue_4 (`GameplayStatics.SpawnEmitterAtLocation` "/Game/Particle/BossProjectileSpawnParticles/P_RingSpawnter.P_RingSpawnter" (`KismetMathLibrary.MakeVector` _returnvalue_x _returnvalue_3 _returnvalue_z) _returnvalue))
  (bind _returnvalue_5 (`GameplayStatics.SpawnEmitterAtLocation` "/Game/Particle/BossProjectileSpawnParticles/P_RingSpawnter.P_RingSpawnter" (`KismetMathLibrary.MakeVector` _returnvalue_x _returnvalue_2 _returnvalue_z) _returnvalue))
  (`KismetSystemLibrary.Delay` 1.0)
  (`|SpawnActorFromClass` "/Game/Inimigos/Boss/BossProjectiles/BP_Projectile02.BP_Projectile02_C" (`KismetMathLibrary.MakeTransform` (`KismetMathLibrary.MakeVector` _returnvalue_x _returnvalue_3 _returnvalue_z) _returnvalue) "Undefined" "OverrideRootScale" null null)
  (`|SpawnActorFromClass` "/Game/Inimigos/Boss/BossProjectiles/BP_Projectile02.BP_Projectile02_C" (`KismetMathLibrary.MakeTransform` (`KismetMathLibrary.MakeVector` _returnvalue_x _returnvalue_2 _returnvalue_z) _returnvalue) "Undefined" "OverrideRootScale" null null)
  (`KismetSystemLibrary.Delay` 0.5)
  (`ActorComponent.K2_DestroyComponent` _returnvalue_5)
  (`ActorComponent.K2_DestroyComponent` _returnvalue_4)
  (set `self.IsAttaking?` false))

(event `self.ReceiveTick`
  (params (DeltaSeconds :type "Float (single-precision)"))
  ;[1 1 1] Seletor aleatório de ataques do Boss
  (if (not (`self.IsAttaking?`))
    (`KismetSystemLibrary.Delay` 1.0)
    (switch `int` (`KismetMathLibrary.RandomIntegerInRange` 0 3)
      (:`0`
        (`self.PAtaque1`))
      (:`1`
        (`self.PAtaque2`))
      (:`2`
        (`self.PAtaque3`)))))

(fn `UserConstructionScript`)