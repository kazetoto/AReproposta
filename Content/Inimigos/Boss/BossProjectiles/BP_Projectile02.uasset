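; Homing boss projectile that chases the player's ship, damages it on capsule overlap and explodes, or despawns after a fixed lifetime.
; Tick traces toward the player pawn until it hits an object, then keeps steering at that cached actor while moving along local forward.
; Turn interpolation speed is inversely proportional to distance, tightening the curve as it closes in.
; Projectile HP logic is unconnected, so incoming damage does nothing.
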(event `self.ReceiveAnyDamage`
  (params (Damage :type "Float (single-precision)") (DamageType :type "DamageType Object Reference") (InstigatedBy :type "Controller Object Reference") (DamageCauser :type "Actor Object Reference"))
  ;[1 1 1] HP do projetil
)

(event `self.Capsule.OnComponentBeginOverlap`
  (params (OverlappedComponent :type "PrimitiveComponent Object Reference") (OtherActor :type "Actor Object Reference") (OtherComp :type "PrimitiveComponent Object Reference") (OtherBodyIndex :type Integer) (bFromSweep :type Boolean) (SweepResult :type "HitResult Structure (by ref)"))
  ;[1 1 1] Aplicar dano somente em player
  (bind _asbp_nave_proposta_2 (cast `/Game/NAVE_PROPOSTA/BP_Nave_Proposta2` OtherActor))
  (`GameplayStatics.ApplyDamage` _asbp_nave_proposta_2 10.0 null self)
  (`GameplayStatics.SpawnEmitterAtLocation` "/Game/StarterContent/Particles/P_Explosion.P_Explosion" (`self.K2_GetActorLocation`) (struct) (1.0 1.0 1.0) false)
  (`self.K2_DestroyActor` self)
  (`KismetSystemLibrary.PrintString` "Player Hited"))

(event `self.ReceiveBeginPlay`
  ;[1 1 1] Despawn
  (`KismetSystemLibrary.Delay` 7.0)
  (`self.K2_DestroyActor`))

(event `self.ReceiveTick`
  (params (DeltaSeconds :type "Float (single-precision)"))
  (bind _returnvalue (`self.K2_GetActorLocation`))
  ;[1 1 1] Projetil segue Player
  (if (stale _returnvalue_3)
    (bind _returnvalue_2 (`self.K2_GetActorLocation` (`.HitActor` (`GameplayStatics.BreakHitResult` (stale _outhit)))))
    (`self.K2_SetActorRotation` (`KismetMathLibrary.RInterpTo` (`self.K2_GetActorRotation`) (`KismetMathLibrary.FindLookAtRotation` _returnvalue _returnvalue_2) DeltaSeconds (* (/ 500.0 (`KismetMathLibrary.VSize` (- _returnvalue _returnvalue_2))) 2.0)) :!label _label)
    (else
      (bind (_outhit _returnvalue_3) (`KismetSystemLibrary.LineTraceSingleForObjects` (`self.K2_GetActorLocation`) (`self.K2_GetActorLocation` (`GameplayStatics.GetPlayerPawn` 0)) (`self.ObejctsToTarget`)))
      (if _returnvalue_3
        (goto _label)
        (else
          _))))
  (`self.K2_AddActorLocalOffset` (`KismetMathLibrary.MakeVector` (* DeltaSeconds 600.0))))

(fn `UserConstructionScript`)