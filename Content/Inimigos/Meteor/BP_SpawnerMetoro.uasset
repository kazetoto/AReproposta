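; Meteor spawner that continuously drops new meteor enemies into the level at an interval set by MeteorFreq.
; After a short startup delay, BeginPlay runs an endless delay loop calling SpawnMeteoro, which cycles through the three meteor classes in order.
; Each meteor spawns at a fixed X and Z with random Y, and one random integer multiplier sets both its scale and Resistencia, so bigger meteors are tougher.
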(event `self.ReceiveBeginPlay`
  (`KismetSystemLibrary.Delay` 0.2)
  (`KismetSystemLibrary.Delay` 1.0)
  (for _ (range 1) :!label _label
    (`self.SpawnMeteoro`)
    (`KismetSystemLibrary.Delay` (`self.MeteorFreq`))
    (goto _label)))

(fn `SpawnMeteoro`
  (bind _fixedrandomvalue (`self.FixedRandomValue`))
  (bind _returnvalue (`KismetMathLibrary.MakeVector` 2500.0 (`KismetMathLibrary.RandomFloatInRange` -900.0 900.0) 400.0))
  (bind _output_get (set `self.FixedRandomValue` (`KismetMathLibrary.RandomIntegerInRange` 1 3)))
  (switch `int` (`self.MeteorSelection`)
    (:`0`
      (bind _returnvalue_2 (* (1.0 1.0 1.0) _output_get))
      (bind _returnvalue_3 (`|SpawnActorFromClass` "/Game/Inimigos/Meteor/BP_Meteor1.BP_Meteor1_C" (`KismetMathLibrary.MakeTransform` _returnvalue (struct) _returnvalue_2) "Undefined" "OverrideRootScale" null null))
      (set `/Game/Inimigos/Meteor/BP_Meteor1.Resistencia` (* _fixedrandomvalue (`/Game/Inimigos/Meteor/BP_Meteor1.Resistencia` _returnvalue_3)) _returnvalue_3)
      (bind _result (`/Engine/EditorBlueprintResources/StandardMacros.IncrementInt` (`self.MeteorSelection`) :!label _label)
        (:`  `
          (set `self.MeteorSelection` _result))))
    (:`1`
      (bind _returnvalue_4 (`|SpawnActorFromClass` "/Game/Inimigos/Meteor/BP_Meteor2.BP_Meteor2_C" (`KismetMathLibrary.MakeTransform` _returnvalue (struct) _returnvalue_2) "Undefined" "OverrideRootScale" null null))
      (set `/Game/Inimigos/Meteor/BP_Meteor2.Resistencia` (* _fixedrandomvalue (`/Game/Inimigos/Meteor/BP_Meteor2.Resistencia` _returnvalue_4)) _returnvalue_4)
      (goto _label))
    (:`2`
      (bind _returnvalue_5 (`|SpawnActorFromClass` "/Game/Inimigos/Meteor/BP_Meteor3.BP_Meteor3_C" (`KismetMathLibrary.MakeTransform` _returnvalue (struct) _returnvalue_2) "Undefined" "OverrideRootScale" null null))
      (set `/Game/Inimigos/Meteor/BP_Meteor3.Resistencia` (* _fixedrandomvalue (`/Game/Inimigos/Meteor/BP_Meteor3.Resistencia` _returnvalue_5)) _returnvalue_5)
      (set `self.MeteorSelection` 0))))

(fn `UserConstructionScript`)