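; Sky backdrop actor for a game map, showing sky and space materials on a Cube mesh.
; On BeginPlay it applies M_Sky_01 to the cube when the MAterial variable is unset or false.
; An unconnected timed sequence, which never runs, would flash seven particle systems to mask swaps to M_Space_01 and, two minutes later, M_Space_02.
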(event `self.ReceiveBeginPlay`
  (if (not (`self.MAterial`))
    (`PrimitiveComponent.SetMaterial` (`self.Cube`) 0 "/Game/Map/M_Sky_01.M_Sky_01")))

(fn `UserConstructionScript`)